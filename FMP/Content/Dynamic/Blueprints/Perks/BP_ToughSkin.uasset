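; BP_ToughSkin is a perk that changes how much damage the player's third-person character takes.
; On apply, it casts the target to BP_ThirdPersonCharacter and multiplies its DamageReistance by the perk's DamageTakenMultiplier.
; On unapply, it divides by the same multiplier to reverse the change, so it adjusts the current value rather than storing the original.
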(event `self.ApplyPerkEffect`
  (params (TargetActor :type "Actor Object Reference"))
  (bind _asbp_third_person_character (cast `/Game/Dynamic/ThirdPerson/Blueprints/BP_ThirdPersonCharacter` TargetActor))
  (set `/Game/Dynamic/ThirdPerson/Blueprints/BP_ThirdPersonCharacter.DamageReistance` (* (`/Game/Dynamic/ThirdPerson/Blueprints/BP_ThirdPersonCharacter.DamageReistance` _asbp_third_person_character) (`self.DamageTakenMultiplier`)) _asbp_third_person_character))

(event `self.UnapplyPerkEffect`
  (params (TargetActor :type "Actor Object Reference"))
  (bind _asbp_third_person_character (cast `/Game/Dynamic/ThirdPerson/Blueprints/BP_ThirdPersonCharacter` TargetActor))
  (set `/Game/Dynamic/ThirdPerson/Blueprints/BP_ThirdPersonCharacter.DamageReistance` (/ (`/Game/Dynamic/ThirdPerson/Blueprints/BP_ThirdPersonCharacter.DamageReistance` _asbp_third_person_character) (`self.DamageTakenMultiplier`)) _asbp_third_person_character))