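; BP_SteadyGrip is a perk Blueprint that modifies the weapon recoil of the third-person player character.
; Applying the perk casts the target to BP_ThirdPersonCharacter and multiplies its Recoil by RecoilMultiplier.
; Unapplying divides Recoil by the same multiplier, reversing the change in place without storing the original value.
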(event `self.ApplyPerkEffect`
  (params (TargetActor :type "Actor Object Reference"))
  ; Apply Steady Grip Perk
  (bind _asbp_third_person_character (cast `/Game/Dynamic/ThirdPerson/Blueprints/BP_ThirdPersonCharacter` TargetActor))
  (set `/Game/Dynamic/ThirdPerson/Blueprints/BP_ThirdPersonCharacter.Recoil` (* (`/Game/Dynamic/ThirdPerson/Blueprints/BP_ThirdPersonCharacter.Recoil` _asbp_third_person_character) (`self.RecoilMultiplier`)) _asbp_third_person_character))

(event `self.UnapplyPerkEffect`
  (params (TargetActor :type "Actor Object Reference"))
  ; Unapply Steady Grip Perk
  (bind _asbp_third_person_character (cast `/Game/Dynamic/ThirdPerson/Blueprints/BP_ThirdPersonCharacter` TargetActor))
  (set `/Game/Dynamic/ThirdPerson/Blueprints/BP_ThirdPersonCharacter.Recoil` (/ (`/Game/Dynamic/ThirdPerson/Blueprints/BP_ThirdPersonCharacter.Recoil` _asbp_third_person_character) (`self.RecoilMultiplier`)) _asbp_third_person_character))