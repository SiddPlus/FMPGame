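; BP_MoreHealth is a perk that raises the maximum health of the player character while it is applied.
; Apply and unapply events cast the target to BP_ThirdPersonCharacter, then add or subtract MaxHealthBonus on its PlayerHealth MaxHealth.
; Only the maximum changes; current health is not adjusted in either direction, and other actor types are ignored.
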(event `self.ApplyPerkEffect`
  (params (TargetActor :type "Actor Object Reference"))
  (bind _asbp_third_person_character (cast `/Game/Dynamic/ThirdPerson/Blueprints/BP_ThirdPersonCharacter` TargetActor))
  (bind _playerhealth (`FMPCharacter.PlayerHealth` _asbp_third_person_character))
  (set `HealthSystem.MaxHealth` (+ (`HealthSystem.MaxHealth` _playerhealth) (`self.MaxHealthBonus`)) _playerhealth))

(event `self.UnapplyPerkEffect`
  (params (TargetActor :type "Actor Object Reference"))
  (bind _asbp_third_person_character (cast `/Game/Dynamic/ThirdPerson/Blueprints/BP_ThirdPersonCharacter` TargetActor))
  (bind _playerhealth (`FMPCharacter.PlayerHealth` _asbp_third_person_character))
  (set `HealthSystem.MaxHealth` (- (`HealthSystem.MaxHealth` _playerhealth) (`self.MaxHealthBonus`)) _playerhealth))