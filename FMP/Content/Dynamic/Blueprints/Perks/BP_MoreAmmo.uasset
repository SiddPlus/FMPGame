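; BP_MoreAmmo is a perk Blueprint that adjusts the MaxAmmo of a BP_ThirdPersonCharacter.
; ApplyPerkEffect casts the target and divides its MaxAmmo by MaxAmmoMultiplier, so only a multiplier below one raises capacity, despite the perk's name.
; UnapplyPerkEffect reverses this by multiplying MaxAmmo by the same value.
; Both events change only the maximum and do nothing for other actor types.
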(event `self.ApplyPerkEffect`
  (params (TargetActor :type "Actor Object Reference"))
  ; Apply More Ammo Perk
  (bind _asbp_third_person_character (cast `/Game/Dynamic/ThirdPerson/Blueprints/BP_ThirdPersonCharacter` TargetActor))
  (set `/Game/Dynamic/ThirdPerson/Blueprints/BP_ThirdPersonCharacter.MaxAmmo` (/ (`/Game/Dynamic/ThirdPerson/Blueprints/BP_ThirdPersonCharacter.MaxAmmo` _asbp_third_person_character) (`self.MaxAmmoMultiplier`)) _asbp_third_person_character))

(event `self.UnapplyPerkEffect`
  (params (TargetActor :type "Actor Object Reference"))
  ; Unapply More Ammo Perk
  (bind _asbp_third_person_character (cast `/Game/Dynamic/ThirdPerson/Blueprints/BP_ThirdPersonCharacter` TargetActor))
  (set `/Game/Dynamic/ThirdPerson/Blueprints/BP_ThirdPersonCharacter.MaxAmmo` (* (`/Game/Dynamic/ThirdPerson/Blueprints/BP_ThirdPersonCharacter.MaxAmmo` _asbp_third_person_character) (`self.MaxAmmoMultiplier`)) _asbp_third_person_character))