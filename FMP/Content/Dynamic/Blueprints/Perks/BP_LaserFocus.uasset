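; Laser Focus perk Blueprint that changes a character's weapon spread while the perk is active.
; On apply, it casts the target to BP_ThirdPersonCharacter and multiplies its Spread by SpreadMultiplier.
; On removal, it divides Spread by the same multiplier to undo the change, doing nothing for other actor types.
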(event `self.ApplyPerkEffect`
  (params (TargetActor :type "Actor Object Reference"))
  ; Apply Laser Focus Perk
  (bind _asbp_third_person_character (cast `/Game/Dynamic/ThirdPerson/Blueprints/BP_ThirdPersonCharacter` TargetActor))
  (set `/Game/Dynamic/ThirdPerson/Blueprints/BP_ThirdPersonCharacter.Spread` (* (`/Game/Dynamic/ThirdPerson/Blueprints/BP_ThirdPersonCharacter.Spread` _asbp_third_person_character) (`self.SpreadMultiplier`)) _asbp_third_person_character))

(event `self.UnapplyPerkEffect`
  (params (TargetActor :type "Actor Object Reference"))
  ; Unapply Laser Focus Perk
  (bind _asbp_third_person_character (cast `/Game/Dynamic/ThirdPerson/Blueprints/BP_ThirdPersonCharacter` TargetActor))
  (set `/Game/Dynamic/ThirdPerson/Blueprints/BP_ThirdPersonCharacter.Spread` (/ (`/Game/Dynamic/ThirdPerson/Blueprints/BP_ThirdPersonCharacter.Spread` _asbp_third_person_character) (`self.SpreadMultiplier`)) _asbp_third_person_character))