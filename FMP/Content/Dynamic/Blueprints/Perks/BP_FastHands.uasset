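; Fast Hands perk Blueprint that changes the player character's reload speed while active.
; Applying the perk casts the target to BP_ThirdPersonCharacter and multiplies its ReloadSpeed by ReloadSpeedMultiplier.
; Unapplying divides by the same multiplier, reversing the change without storing the original value.
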(event `self.ApplyPerkEffect`
  (params (TargetActor :type "Actor Object Reference"))
  ; Apply Fast Hands Perk
  (bind _asbp_third_person_character (cast `/Game/Dynamic/ThirdPerson/Blueprints/BP_ThirdPersonCharacter` TargetActor))
  (set `/Game/Dynamic/ThirdPerson/Blueprints/BP_ThirdPersonCharacter.ReloadSpeed` (* (`/Game/Dynamic/ThirdPerson/Blueprints/BP_ThirdPersonCharacter.ReloadSpeed` _asbp_third_person_character) (`self.ReloadSpeedMultiplier`)) _asbp_third_person_character))

(event `self.UnapplyPerkEffect`
  (params (TargetActor :type "Actor Object Reference"))
  ; Unapply Fast Hands Perk
  (bind _asbp_third_person_character (cast `/Game/Dynamic/ThirdPerson/Blueprints/BP_ThirdPersonCharacter` TargetActor))
  (set `/Game/Dynamic/ThirdPerson/Blueprints/BP_ThirdPersonCharacter.ReloadSpeed` (/ (`/Game/Dynamic/ThirdPerson/Blueprints/BP_ThirdPersonCharacter.ReloadSpeed` _asbp_third_person_character) (`self.ReloadSpeedMultiplier`)) _asbp_third_person_character))