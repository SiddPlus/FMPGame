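; Perk Blueprint that makes the player's hits slow enemies.
; Applying the perk binds a handler to the third-person character's OnEnemyHit event, and unapplying it unbinds that handler.
; Each hit on a BP_Enemy subtracts a slow amount from its MaxWalkSpeed, so slows stack with no clamp, timer or restore in this graph.
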(event `self.ApplyPerkEffect`
  (params (TargetActor :type "Actor Object Reference"))
  (bind _asbp_third_person_character (cast `/Game/Dynamic/ThirdPerson/Blueprints/BP_ThirdPersonCharacter` TargetActor))
  (add `/Game/Dynamic/ThirdPerson/Blueprints/BP_ThirdPersonCharacter.OnEnemyHit` _asbp_third_person_character (delegate `Enemy Hit`)))

(event `Enemy Hit`
  (params (Enemy :type "Actor Object Reference"))
  (bind _asbp_enemy (cast `/Game/Dynamic/Blueprints/AI/BP_Enemy` Enemy))
  (bind _charactermovement (`Character.CharacterMovement` _asbp_enemy))
  (set `CharacterMovementComponent.MaxWalkSpeed` (- (`CharacterMovementComponent.MaxWalkSpeed` _charactermovement) (`self.EnemySlowAmmount`)) _charactermovement))

(event `self.UnapplyPerkEffect`
  (params (TargetActor :type "Actor Object Reference"))
  (bind _asbp_third_person_character (cast `/Game/Dynamic/ThirdPerson/Blueprints/BP_ThirdPersonCharacter` TargetActor))
  (remove `/Game/Dynamic/ThirdPerson/Blueprints/BP_ThirdPersonCharacter.OnEnemyHit` _asbp_third_person_character (delegate `Enemy Hit`)))