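; BP_ToughToKill is a perk that gives the player character passive health regeneration.
; Applying it sets a regen flag, caches the target as BP_ThirdPersonCharacter and starts a looping one-second timer.
; Each tick raises health by HealthRegenAmount through PlayerHealth while the flag is set and the character is alive.
; Unapplying only clears the flag, leaving the timer running.
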(event `self.ApplyPerkEffect`
  (params (TargetActor :type "Actor Object Reference"))
  (set `self.Regen` true)
  (bind _asbp_third_person_character (cast `/Game/Dynamic/ThirdPerson/Blueprints/BP_ThirdPersonCharacter` TargetActor))
  (`KismetSystemLibrary.K2_SetTimerDelegate` (delegate `RegenTick`) 1.0 true))

(event `RegenTick`
  (if (`self.Regen`)
    (if (not (`/Game/Dynamic/ThirdPerson/Blueprints/BP_ThirdPersonCharacter.Dead` (stale `self.ApplyPerkEffect` _asbp_third_person_character)))
      (`HealthSystem.IncreaseHealth` (`FMPCharacter.PlayerHealth` (stale `self.ApplyPerkEffect` _asbp_third_person_character)) (`self.HealthRegenAmount`)))))

(event `self.UnapplyPerkEffect`
  (params (TargetActor :type "Actor Object Reference"))
  (set `self.Regen` false))