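; A perk Blueprint that raises the damage of the third-person player character while it is active.
; Applying the perk casts the target to BP_ThirdPersonCharacter and multiplies its Damage by DamageMultiplier.
; Unapplying it divides Damage by the same multiplier, and both events do nothing for other actor types.
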(event `self.ApplyPerkEffect`
  (params (TargetActor :type "Actor Object Reference"))
  ; Apply More Damage Perk
  (bind _asbp_third_person_character (cast `/Game/Dynamic/ThirdPerson/Blueprints/BP_ThirdPersonCharacter` TargetActor))
  (set `/Game/Dynamic/ThirdPerson/Blueprints/BP_ThirdPersonCharacter.Damage` (* (`/Game/Dynamic/ThirdPerson/Blueprints/BP_ThirdPersonCharacter.Damage` _asbp_third_person_character) (`self.DamageMultiplier`)) _asbp_third_person_character))

(event `self.UnapplyPerkEffect`
  (params (TargetActor :type "Actor Object Reference"))
  ; Unapply More Damage Perk
  (bind _asbp_third_person_character (cast `/Game/Dynamic/ThirdPerson/Blueprints/BP_ThirdPersonCharacter` TargetActor))
  (set `/Game/Dynamic/ThirdPerson/Blueprints/BP_ThirdPersonCharacter.Damage` (/ (`/Game/Dynamic/ThirdPerson/Blueprints/BP_ThirdPersonCharacter.Damage` _asbp_third_person_character) (`self.DamageMultiplier`)) _asbp_third_person_character))