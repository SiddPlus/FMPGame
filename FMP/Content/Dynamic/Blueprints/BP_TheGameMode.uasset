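; BP_TheGameMode is the game mode that switches background music between idle and combat tracks based on round state.
; On BeginPlay it spawns both 2D tracks, binds to the game state's OnRoundStateChange event, and applies the inactive state.
; Each round state change crossfades between the tracks, fading combat music in when a round is active and idle music in otherwise.
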(event `self.ReceiveBeginPlay`
  (bind _asbp_the_game_state (cast `/Game/Dynamic/Blueprints/BP_TheGameState` (`GameplayStatics.GetGameState`)))
  (set `self.As BP The Game State` _asbp_the_game_state)
  (bind _returnvalue (`GameplayStatics.SpawnSound2D` "/Game/Static/Sound/Music/SFX_Idle.SFX_Idle" 1.0 1.0 0.0 null))
  (set `self.IdleMusic` _returnvalue)
  (bind _returnvalue_2 (`GameplayStatics.SpawnSound2D` "/Game/Static/Sound/Music/SFX_CombatMusic.SFX_CombatMusic" 1.0 1.0 0.0 null))
  (set `self.CombatMusic` _returnvalue_2)
  (add `TheGameState.OnRoundStateChange` (`self.As BP The Game State`) (delegate `RoundStateChange`))
  (`self.RoundStateChange` false))

(event `RoundStateChange`
  (params (IsActive :type Boolean))
  (if IsActive
    (`AudioComponent.FadeIn` (`self.CombatMusic`) 2.0 1.0 0.0 "Linear")
    (`AudioComponent.FadeOut` (`self.IdleMusic`) 2.0 0.0 "Linear")
    (else
      (`AudioComponent.FadeIn` (`self.IdleMusic`) 2.0 1.0 0.0 "Linear")
      (`AudioComponent.FadeOut` (`self.CombatMusic`) 2.0 0.0 "Linear"))))

(event `self.ReceiveTick`
  (params (DeltaSeconds :type "Float (single-precision)")))

(fn `UserConstructionScript`)