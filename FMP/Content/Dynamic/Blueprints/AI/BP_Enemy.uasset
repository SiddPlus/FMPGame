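; Enemy AI actor that attacks players and dies when its health runs out.
; Health changes drive a dead flag and delayed destruction, while attack events play a montage and store the target.
; A separate damage event scales base damage by round number and player count from the game state, then applies the player's resistance multiplier.
; If SprintBurst is set, the hit player's walk speed is temporarily overridden, then restored.
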(event `self.ReceiveBeginPlay`
  (add `HealthSystem.OnHealthChanged` (`self.GetComponentByClass` "/Script/FMP.HealthSystem") (delegate `Update`)))

(event `Update`
  (params (HealthComp :type "HealthSystem Object Reference") (Health :type "Float (single-precision)") (HealthDelta :type "Float (single-precision)") (DamageType :type "DamageType Object Reference"))
  (if (<= (`HealthSystem.CurrentHealth` (`self.EnemyHealth`)) 0.0)
    (set `self.Dead` true)
    (`KismetSystemLibrary.Delay` 5.0)
    (`self.K2_DestroyActor`)))

(event `ServerPerformAttack`
  (params (TargetActor :type "Actor Object Reference"))
  (set `self.Target Actor` TargetActor)
  (bind _returnvalue (`self.PlayAnimMontage` "/Game/Dynamic/Enemy/AM_Attack.AM_Attack"))
  (`KismetSystemLibrary.Delay` _returnvalue))

(event `SeverApplyDamage`
  (bind _charactermovement (`Character.CharacterMovement` (`self.As BP Third Person Character`)))
  (`self.SeverCalculateDamage`)
  (bind _asbp_third_person_character (cast `/Game/Dynamic/ThirdPerson/Blueprints/BP_ThirdPersonCharacter` (`self.Target Actor`)))
  (bind _output_get (set `self.As BP Third Person Character` _asbp_third_person_character))
  (`HealthSystem.DecreaseHealth` (`FMPCharacter.PlayerHealth` _output_get) (* (`self.NewDamage`) (`/Game/Dynamic/ThirdPerson/Blueprints/BP_ThirdPersonCharacter.DamageReistance` _asbp_third_person_character)) null)
  (if (`self.SprintBurst`)
    (set `self.Player Max Speed` (`CharacterMovementComponent.MaxWalkSpeed` _charactermovement))
    (set `CharacterMovementComponent.MaxWalkSpeed` 900.0 _charactermovement)
    (`KismetSystemLibrary.Delay` 5.0)
    (set `CharacterMovementComponent.MaxWalkSpeed` (`self.Player Max Speed`) (`Character.CharacterMovement` (`self.As BP Third Person Character`)))))

(event `SeverCalculateDamage`
  (bind _asbp_the_game_state (cast `/Game/Dynamic/Blueprints/BP_TheGameState` (`GameplayStatics.GetGameState`)))
  (set `self.NewDamage` (* (* (+ (* (- (`TheGameState.CurrentRoundNumber` _asbp_the_game_state) 1) 0.1) 1.0) (+ (* (- (`TheGameState.TotalPlayersInGame` _asbp_the_game_state) 1) 0.2) 1.0)) (`self.BaseDamage`))))

(fn `UserConstructionScript`)